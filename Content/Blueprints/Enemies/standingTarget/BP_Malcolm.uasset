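; BP_Malcolm is a standing-target enemy that reacts when shot by a BP_Projectile.
; The construction script attaches separate Head and Body hit components to the mesh's Head and Hips sockets.
; A projectile hit on either component calls TorsoShot on the ABP_Malcolm anim instance, so head hits currently trigger the same reaction as body hits.
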(event OnComponentHit(Body)
  (params (HitComponent :type Primitive%20Component%20Object%20Reference) (OtherActor :type Actor%20Object%20Reference) (OtherComp :type Primitive%20Component%20Object%20Reference) (NormalImpulse :type Vector :default "0, 0, 0") (Hit :type Hit%20Result%20Structure%20%28by%20ref%29))
  (Utilities|Casting|CastToBP_Projectile OtherActor)
  (bind _asabp_malcolm (Utilities|Casting|CastToABP_Malcolm (Components|SkeletalMesh|GetAnimInstance (Variables|Character|GetMesh))))
  (Default|TorsoShot _asabp_malcolm))

(event OnComponentHit(Head)
  (params (HitComponent :type Primitive%20Component%20Object%20Reference) (OtherActor :type Actor%20Object%20Reference) (OtherComp :type Primitive%20Component%20Object%20Reference) (NormalImpulse :type Vector :default "0, 0, 0") (Hit :type Hit%20Result%20Structure%20%28by%20ref%29))
  (Utilities|Casting|CastToBP_Projectile OtherActor)
  (bind _asabp_malcolm (Utilities|Casting|CastToABP_Malcolm (Components|SkeletalMesh|GetAnimInstance (Variables|Character|GetMesh))))
  (Default|TorsoShot _asabp_malcolm))

(fn ConstructionScript
  (Transformation|AttachComponentToComponent (Variables|Default|GetHead) (Variables|Character|GetMesh) "Head" "KeepRelative" "KeepRelative" "KeepRelative" true)
  (Transformation|AttachComponentToComponent (Variables|Default|GetBody) (Variables|Character|GetMesh) "Hips" "KeepRelative" "KeepRelative" "KeepRelative" true))