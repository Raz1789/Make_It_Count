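; BP_NPC_Liam is an enemy NPC character that dies when its capsule is hit by a BP_Projectile.
; The hit sets the Death flag on its ABP_NPC_Liam anim instance and stops current movement immediately, with no health or damage calculation.
; The construction script attaches a static mesh to the RightHandMiddle1 socket on the skeletal mesh, keeping its relative transform.
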(event OnComponentHit(CapsuleComponent)
  (params (HitComponent :type Primitive%20Component%20Object%20Reference) (OtherActor :type Actor%20Object%20Reference) (OtherComp :type Primitive%20Component%20Object%20Reference) (NormalImpulse :type Vector :default "0, 0, 0") (Hit :type Hit%20Result%20Structure%20%28by%20ref%29))
  (Utilities|Casting|CastToBP_Projectile OtherActor)
  (bind _asabp_npc_liam (Utilities|Casting|CastToABP_NPC_Liam (Components|SkeletalMesh|GetAnimInstance (Variables|Character|GetMesh))))
  (Variables|/Game/Blueprints/Enemies/NPCs/Liam/ABP_NPC_Liam.ABP_NPC_Liam_C|SetbDeath _asabp_npc_liam true)
  (Components|Movement|StopMovementImmediately (Variables|Character|GetCharacterMovement)))

(fn ConstructionScript
  (Transformation|AttachComponentToComponent (Variables|Default|GetStaticMesh) (Variables|Character|GetMesh) "RightHandMiddle1" "KeepRelative" "KeepRelative" "KeepRelative" true))