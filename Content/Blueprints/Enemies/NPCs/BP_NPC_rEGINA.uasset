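; NPC character Regina, which walks to a set location and dies when hit by a projectile.
; Two seconds after BeginPlay, an AI move sends it toward MoveToLocation.
; A capsule hit from BP_Projectile sets the Death flag on its ABP_NPC_Regina anim instance and calls StopMovementImmediately on its movement component.
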(event OnComponentHit(CapsuleComponent)
  (params (HitComponent :type Primitive%20Component%20Object%20Reference) (OtherActor :type Actor%20Object%20Reference) (OtherComp :type Primitive%20Component%20Object%20Reference) (NormalImpulse :type Vector :default "0, 0, 0") (Hit :type Hit%20Result%20Structure%20%28by%20ref%29))
  (Utilities|Casting|CastToBP_Projectile OtherActor)
  (bind _asabp_npc_regina (Utilities|Casting|CastToABP_NPC_Regina (Components|SkeletalMesh|GetAnimInstance (Variables|Character|GetMesh))))
  (Variables|/Game/Blueprints/Enemies/NPCs/Regina/ABP_NPC_Regina.ABP_NPC_Regina_C|SetbDeath _asabp_npc_regina true)
  (Components|Movement|StopMovementImmediately (Variables|Character|GetCharacterMovement)))

(event EventBeginPlay
  (Utilities|FlowControl|Delay 2.0)
  (AI|AIMoveTo self (Variables|Default|GetMoveToLocation) 0 5.0 false))

(fn ConstructionScript)