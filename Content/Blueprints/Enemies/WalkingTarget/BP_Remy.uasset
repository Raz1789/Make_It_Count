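; Remy walking-target enemy that moves to a set location via AI MoveTo two seconds after BeginPlay.
; Construction script attaches Head and Body hit components to the mesh's Head and Hips sockets so they follow the skeleton.
; A BP_Projectile hit on either component sets the Death flag in ABP_NPC_Remy and stops current movement, with no difference between head and body hits.
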(event OnComponentHit(Body)
  (params (HitComponent :type Primitive%20Component%20Object%20Reference) (OtherActor :type Actor%20Object%20Reference) (OtherComp :type Primitive%20Component%20Object%20Reference) (NormalImpulse :type Vector :default "0, 0, 0") (Hit :type Hit%20Result%20Structure%20%28by%20ref%29))
  (Utilities|Casting|CastToBP_Projectile OtherActor)
  (bind _asabp_npc_remy (Utilities|Casting|CastToABP_NPC_Remy (Components|SkeletalMesh|GetAnimInstance (Variables|Character|GetMesh))))
  (Variables|/Game/Blueprints/Enemies/NPCs/Remy/ABP_NPC_Remy.ABP_NPC_Remy_C|SetbDeath _asabp_npc_remy true)
  (Components|Movement|StopMovementImmediately (Variables|Character|GetCharacterMovement)))

(event OnComponentHit(Head)
  (params (HitComponent :type Primitive%20Component%20Object%20Reference) (OtherActor :type Actor%20Object%20Reference) (OtherComp :type Primitive%20Component%20Object%20Reference) (NormalImpulse :type Vector :default "0, 0, 0") (Hit :type Hit%20Result%20Structure%20%28by%20ref%29))
  (Utilities|Casting|CastToBP_Projectile OtherActor)
  (bind _asabp_npc_remy (Utilities|Casting|CastToABP_NPC_Remy (Components|SkeletalMesh|GetAnimInstance (Variables|Character|GetMesh))))
  (Variables|/Game/Blueprints/Enemies/NPCs/Remy/ABP_NPC_Remy.ABP_NPC_Remy_C|SetbDeath _asabp_npc_remy true)
  (Components|Movement|StopMovementImmediately (Variables|Character|GetCharacterMovement)))

(event EventBeginPlay
  (Utilities|FlowControl|Delay 2.0)
  (AI|AIMoveTo self (Variables|Default|GetMoveToLocation) 0 5.0 false))

(fn ConstructionScript
  (Transformation|AttachComponentToComponent (Variables|Default|GetHead) (Variables|Character|GetMesh) "Head" "KeepRelative" "KeepRelative" "KeepRelative" true)
  (Transformation|AttachComponentToComponent (Variables|Default|GetBody) (Variables|Character|GetMesh) "Hips" "KeepRelative" "KeepRelative" "KeepRelative" true))