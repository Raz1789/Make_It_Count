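; BP_Liam is an enemy NPC, filed under RandomWalk, that dies when struck by a projectile.
; The construction script attaches Head and Body hit components and a Phone to skeleton sockets on the mesh.
; A BP_Projectile hit on either Head or Body sets the Death flag on the ABP_NPC_Liam animation blueprint, with no damage or health logic.
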(event OnComponentHit(Body)
  (params (HitComponent :type Primitive%20Component%20Object%20Reference) (OtherActor :type Actor%20Object%20Reference) (OtherComp :type Primitive%20Component%20Object%20Reference) (NormalImpulse :type Vector :default "0, 0, 0") (Hit :type Hit%20Result%20Structure%20%28by%20ref%29))
  (Utilities|Casting|CastToBP_Projectile OtherActor)
  (bind _asabp_npc_liam (Utilities|Casting|CastToABP_NPC_Liam (Components|SkeletalMesh|GetAnimInstance (Variables|Character|GetMesh))))
  (Variables|/Game/Blueprints/Enemies/NPCs/Liam/ABP_NPC_Liam.ABP_NPC_Liam_C|SetbDeath _asabp_npc_liam true))

(event OnComponentHit(Head)
  (params (HitComponent :type Primitive%20Component%20Object%20Reference) (OtherActor :type Actor%20Object%20Reference) (OtherComp :type Primitive%20Component%20Object%20Reference) (NormalImpulse :type Vector :default "0, 0, 0") (Hit :type Hit%20Result%20Structure%20%28by%20ref%29))
  (Utilities|Casting|CastToBP_Projectile OtherActor)
  (bind _asabp_npc_liam (Utilities|Casting|CastToABP_NPC_Liam (Components|SkeletalMesh|GetAnimInstance (Variables|Character|GetMesh))))
  (Variables|/Game/Blueprints/Enemies/NPCs/Liam/ABP_NPC_Liam.ABP_NPC_Liam_C|SetbDeath _asabp_npc_liam true))

(fn ConstructionScript
  (Transformation|AttachComponentToComponent (Variables|Default|GetHead) (Variables|Character|GetMesh) "Head" "KeepRelative" "KeepRelative" "KeepRelative" true)
  (Transformation|AttachComponentToComponent (Variables|Default|GetBody) (Variables|Character|GetMesh) "Hips" "KeepRelative" "KeepRelative" "KeepRelative" true)
  (Transformation|AttachComponentToComponent (Variables|Default|Getphone) (Variables|Character|GetMesh) "RightHandMiddle1" "KeepRelative" "KeepRelative" "KeepRelative" true))