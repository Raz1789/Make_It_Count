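; BP_Projectile is a projectile with its own camera that reports where it strikes an enemy.
; On hit, it ignores the player and other projectiles, and prints head, torso or miss for BP_Enemy by comparing the hit component.
; Any other hit, enemies included, destroys the mesh and stops movement.
; Tick then slides the camera along world X for up to 100 frames; a mesh rotation snippet is left unconnected.
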(event OnComponentHit(collision)
  (params (HitComponent :type Primitive%20Component%20Object%20Reference) (OtherActor :type Actor%20Object%20Reference) (OtherComp :type Primitive%20Component%20Object%20Reference) (NormalImpulse :type Vector :default "0, 0, 0") (Hit :type Hit%20Result%20Structure%20%28by%20ref%29))
  (bind _projectilemovement (Variables|Default|GetProjectileMovement))
  (Variables|Default|SetOtherActor OtherActor)
  (Variables|Default|SetOtherComp OtherComp)
  (Utilities|Casting|CastToBP_PlayerCharacter (Variables|Default|GetOtherActor)
    (:CastFailed
      (Utilities|Casting|CastToBP_Projectile (Variables|Default|GetOtherActor)
        (:CastFailed
          (Utilities|FlowControl|Sequence
            (:then_0
              (bind _asbp_enemy (Utilities|Casting|CastToBP_Enemy (Variables|Default|GetOtherActor)))
              (Development|PrintString (Utilities|GetDisplayName (Variables|Default|GetOtherComp)))
              (if (== (Variables|Default|GetOtherComp) (Variables|/Game/Blueprints/Enemies/BP_Enemy.BP_Enemy_C|GetHead _asbp_enemy))
                (Development|PrintString "Head Shot")
                (elif (== (Variables|/Game/Blueprints/Enemies/BP_Enemy.BP_Enemy_C|GetBody _asbp_enemy) (Variables|Default|GetOtherComp))
                  (Development|PrintString "Torso Shot")
                  (else
                    (Development|PrintString "Target Missed")))))
            (:then_1
              (Components|DestroyComponent (Variables|Default|GetProjectileMesh))
              (Game|Components|ProjectileMovement|StopSimulating _projectilemovement Hit)
              (Components|Movement|StopMovementImmediately _projectilemovement))))))))

(event EventTick
  (params (DeltaSeconds :type Float%20%28single-precision%29))
  (bind _projectilecamera (Variables|Default|GetProjectileCamera))
  (bind _returnvalue (Transformation|GetWorldLocation _projectilecamera))
  (Utilities|IsValid (Variables|Default|GetProjectileMesh)
    (:Is%20Not%20Valid
      (Utilities|FlowControl|DoN 100
        (:Exit
          (Transformation|SetWorldLocation _projectilecamera (Math|Vector|MakeVector (+ (.x _returnvalue) (* DeltaSeconds (Variables|Default|GetCamMoveRate))) (.y _returnvalue) (.z _returnvalue)) false false))))))

(fn ConstructionScript)